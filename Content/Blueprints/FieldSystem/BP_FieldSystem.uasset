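; Field system actor that fires a one-shot radial burst at its location when play begins, to break and scatter Chaos destructible objects.
; BeginPlay calls CreateField, which applies a no-falloff radial external cluster strain within a sphere, then a radial vector linear force with a metadata filter.
; An unconnected, near-identical copy of this field chain remains in the event graph and never runs.
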(event `self.ReceiveBeginPlay`
  (`self.CreateField`))

(fn `CreateField`
  (bind _returnvalue (`self.K2_GetActorLocation`))
  (bind _fieldsystemcomponent (`self.FieldSystemComponent`))
  (`FieldSystemComponent.ApplyPhysicsField` _fieldsystemcomponent true "Field_ExternalClusterStrain" null (`RadialFalloff.SetRadialFalloff` (`self.RadialFalloff`) 1000000.0 1.0 1.0 0.0 200.0 _returnvalue "Field_FallOff_None"))
  (`FieldSystemComponent.ApplyPhysicsField` _fieldsystemcomponent true "Field_LinearForce" (`self.FieldSystemMetaDataFilter`) (`RadialVector.SetRadialVector` (`self.RadialVector`) 900000.0 _returnvalue)))

(fn `UserConstructionScript`)