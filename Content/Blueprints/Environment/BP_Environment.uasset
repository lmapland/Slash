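; BP_Environment drives the day-night cycle and switches the ambient music between day and night.
; On BeginPlay it finds the tagged sun and night directional lights and the BP_AmbientMusic actor, then starts daytime music.
; Tick pitches both lights at CycleSpeed and watches the sun's rotation for the two horizon crossings.
; A pair of DoOnce gates reset each other, so each crossing calls SetTimeOfDay only once.
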(event `self.ReceiveBeginPlay`
  (bind _outactors (`GameplayStatics.GetAllActorsOfClassWithTag` "/Script/Engine.DirectionalLight" "SunLight"))
  (set `self.SunLight` (`|GetArrayItem` _outactors))
  (bind _outactors_2 (`GameplayStatics.GetAllActorsOfClassWithTag` "/Script/Engine.DirectionalLight" "NightLight"))
  (set `self.NightLight` (`|GetArrayItem` _outactors_2))
  (bind _outactors_3 (`GameplayStatics.GetAllActorsOfClassWithTag` "/Game/Blueprints/Environment/BP_AmbientMusic.BP_AmbientMusic_C" "AmbientMusic"))
  (bind _output_get (set `self.MusicPlayer` (`|GetArrayItem` _outactors_3)))
  (`/Game/Blueprints/Environment/BP_AmbientMusic.Setup` _output_get true 0)
  (`/Game/Blueprints/Environment/BP_AmbientMusic.PlayMusic` _output_get))

(event `self.ReceiveTick`
  (params (DeltaSeconds :type "Float (single-precision)"))
  (bind _returnvalue (`self.K2_GetActorRotation` (`self.SunLight`)))
  (bind _returnvalue_2 (`KismetMathLibrary.MakeRotator` 0.0 (* DeltaSeconds (`self.CycleSpeed`))))
  (`self.K2_AddActorLocalRotation` (`self.SunLight`) _returnvalue_2 false false)
  (`self.K2_AddActorLocalRotation` (`self.NightLight`) _returnvalue_2 false false)
  ;[1 1 1] Day -> Night
  (if (== _returnvalue (struct) :`ErrorTolerance` 1.0)
    (`/Engine/EditorBlueprintResources/StandardMacros.DoOnce` false :!label _label
      (:`Completed`
        (`|ExecutionSequence`
          (:`then_0`
            (`KismetSystemLibrary.PrintString` "BP_Environment: Called SetTimeOfDay(17)")
            (`/Game/Blueprints/Environment/BP_AmbientMusic.SetTimeOfDay` (`self.MusicPlayer`) 17))
          (:`then_1`
            (goto _label_2 :!via `Reset`)))))
    (else
      ;[1 1 1] Night -> Day
      (if (== _returnvalue (struct :`Yaw` 180.0 :`Roll` 180.0) :`ErrorTolerance` 1.0)
        (`/Engine/EditorBlueprintResources/StandardMacros.DoOnce` false :!label _label_2
          (:`Completed`
            (`|ExecutionSequence`
              (:`then_0`
                (`KismetSystemLibrary.PrintString` "BP_Environment: Called SetTimeOfDay(6)")
                (`/Game/Blueprints/Environment/BP_AmbientMusic.SetTimeOfDay` (`self.MusicPlayer`) 6))
              (:`then_1`
                (goto _label :!via `Reset`)))))))))

(fn `UserConstructionScript`)