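; BP_AmbientMusic is an actor that drives ambient music based on time of day.
; Setup spawns a 2D MetaSound and stores the day/night state and weather, though weather does not yet affect the music.
; SetTimeOfDay treats 6 to 17 as day and, only when day and night flip, selects a new trigger name.
; PlayMusic sends that trigger to the MetaSound, which must define matching triggers.
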(fn `PlayMusic`
  (bind _triggername (`self.TriggerName`))
  (`KismetSystemLibrary.PrintString` "PlayMusic(): Beginning to play music now")
  (`KismetSystemLibrary.PrintString` (`KismetStringLibrary.Conv_NameToString` _triggername))
  (`AudioParameterControllerInterface.SetTriggerParameter` (`self.Target`) _triggername))

(fn `SetTimeOfDay`
  (params (InTimeOfDay :type Integer))
  (bind _output_get (set `self.TimeOfDay` InTimeOfDay))
  ;[1 1 1] Is the new time Night?
  (if (or (>= _output_get 17) (< _output_get 6))
    ;[1 1 1] New time is Night, current time is Day
    (if (`self.IsDaytime`)
      (`KismetSystemLibrary.PrintString` "In SetTimeOfDay(): New time is night, current time is day - changing trigger name and playing music")
      (set `self.IsDaytime` false)
      (`self.SetTriggerName` :!label _label)
      (`self.PlayMusic`)
      (else
        (`KismetSystemLibrary.PrintString` "In SetTimeOfDay(): New time is night, current time is night - doing nothing")))
    (else
      ;[1 1 1] New time is Day, current time is Night
      (if (`self.IsDaytime`)
        (`KismetSystemLibrary.PrintString` "In SetTimeOfDay(): New time is day, current time is day- doing nothing")
        (else
          (`KismetSystemLibrary.PrintString` "In SetTimeOfDay(): New time is day, current time is night- changing trigger name and playing music")
          (set `self.IsDaytime` true)
          (goto _label))))))

(fn `SetTriggerName`
  ;[1 1 1] So far only takes into account daytime vs nighttime; will eventually take weather patterns into account. Updates to this function require equal updates to the MetaSound so it can process the new / updated trigger
  (if (`self.IsDaytime`)
    (set `self.TriggerName` (`self.TriggerSunnyDay`))
    (else
      (set `self.TriggerName` (`self.TriggerNight`)))))

(fn `Setup`
  (params (bIsDaytime :type Boolean) (Weather :type Integer))
  ;[1 1 1] Weather: 0 = sunny, 1 = breezy, 2 = light rain, 3 = heavy rain, 4 = storm, 5 = light fog, 6 = heavy fog, 7 = light snow, 8 = heavy snow, 9 = blizzard
  (set `self.IsDaytime` bIsDaytime)
  (set `self.CurrentWeather` Weather)
  (`self.SetTriggerName`)
  (bind _returnvalue (`GameplayStatics.SpawnSound2D` (`self.DayMusic`) 1.0 1.0 0.0 null))
  (set `self.Target` _returnvalue))

(fn `UserConstructionScript`)