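; Patrol mob spawner, named DONOTUSE, that spawns one random stag or wolf variant on BeginPlay and starts it patrolling.
; Spawn positions are random points in a box, snapped to ground by a downward object line trace.
; It scatters up to five TargetPoints around the enemy's spawn location and adds them to its PatrolPoints.
; A random one becomes PatrolTarget before StartPatrolling; a failed enemy ground trace only logs.
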(event `self.ReceiveBeginPlay`
  (bind _enemyobject (`self.EnemyObject`))
  (set `self.ChosenEnemy` (`KismetArrayLibrary.Array_Random` (`|MakeArray` (`self.StagRef`) (`self.StagRedRef`) (`self.WolfRef`) (`self.WolfieRef`) :!type "/Game/Blueprints/Enemies/BP_Enemy Class Reference")))
  ;[1 1 1] Choose location for Enemy; make sure it spawns on the ground and spawn it
  (bind (_spawntransform _valid) (`self.GetTargetSpawnLocation` (`self.K2_GetActorLocation`) (`self.EnemySpawnHalfSize`)))
  (if _valid
    (`KismetSystemLibrary.LogString` "LineTrace for PatrolEnemy got a hit")
    (bind _output_get (set `self.ChosenPoint` _spawntransform))
    (bind _returnvalue (`|SpawnActorFromClass` (`self.ChosenEnemy`) _output_get "AdjustIfPossibleButAlwaysSpawn" "OverrideRootScale" null null))
    (set `self.EnemyObject` _returnvalue)
    (for _index (range 1 6)
      (if (> _index 5)
        (break)
        (else
          ;[1 1 1] Create and add Patrol Point (Target Point) to Enemy
          (bind (_spawntransform_2 _valid_2) (`self.GetTargetSpawnLocation` (+ (.location (`self.ChosenPoint`)) (0.0 0.0 200.0)) (`self.TargetSpawnHalfSize`)))
          (if _valid_2
            (bind _returnvalue_2 (`|SpawnActorFromClass` "/Script/Engine.TargetPoint" _spawntransform_2 "AdjustIfPossibleButAlwaysSpawn" "OverrideRootScale" null null))
            (`KismetArrayLibrary.Array_Add` (`Enemy.PatrolPoints` (`self.EnemyObject`)) _returnvalue_2)
            (else
              (`KismetSystemLibrary.PrintString` "PatrolTarget did not spawn"))))))
    (`KismetSystemLibrary.PrintString` "Done with the loop; going to call StartPatrolling()")
    (set `Enemy.PatrolTarget` (`KismetArrayLibrary.Array_Random` (`Enemy.PatrolPoints` _enemyobject)) _enemyobject)
    (`Enemy.StartPatrolling` _enemyobject)
    (else
      (`KismetSystemLibrary.LogString` "LineTrace for PatrolEnemy DID NOT get a hit"))))

(fn `GetTargetSpawnLocation`
  (params (Origin :type "Vector Structure") (HalfSize :type "Vector Structure"))
  (returns (SpawnTransform :type "Transform Structure") (Valid :type Boolean))
  (locals (SpawnPoint :type "Vector Structure"))
  (bind _output_get (set `local.SpawnPoint` (`KismetMathLibrary.RandomPointInBoundingBox` Origin HalfSize)))
  (bind (_z _found_ground) (`self.GetZOnGround` _output_get))
  (return (`KismetMathLibrary.MakeTransform` (`KismetMathLibrary.MakeVector` (.x _output_get) (.y _output_get) _z)) _found_ground))

(fn `GetZOnGround`
  (params (Origin :type "Vector Structure"))
  (returns (Z :type "Float (double-precision)") (`Found ground` :type Boolean))
  (bind (_outhit _returnvalue) (`KismetSystemLibrary.LineTraceSingleForObjects` :`Start` Origin :`End` (- Origin (0.0 0.0 600.0)) :`ObjectTypes` (`self.LineTraceObjectType`) :`DrawTime` 0.0))
  (return (.z (`.ImpactPoint` (`GameplayStatics.BreakHitResult` _outhit))) _returnvalue))

(fn `UserConstructionScript`)