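; BP_FlowerSpawner scatters BP_RaspberryNode actors across the area around itself, despite its flower name.
; Shortly after BeginPlay, it loops over a fixed number of attempts, picking random points in a wide, flat box centered on its location.
; Each point gets a downward object line trace, and a hit spawns a node at that height, adjusting for collisions but always spawning.
; Missed traces are skipped without retry.
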(event `self.ReceiveBeginPlay`
  (`KismetSystemLibrary.Delay` 0.1)
  (for _index (range 1 26)
    (if (> _index 26)
      (break)
      (else
        (bind _output_get (set `self.ChosenPoint` (`KismetMathLibrary.RandomPointInBoundingBox` (`self.K2_GetActorLocation`) (4000.0 4000.0 0.0))))
        (bind (_outhit _returnvalue) (`KismetSystemLibrary.LineTraceSingleForObjects` :`Start` _output_get :`End` (- (`self.ChosenPoint`) (0.0 0.0 600.0)) :`ObjectTypes` (`self.LineTraceObjectType`) :`DrawTime` 0.0))
        (if _returnvalue
          (`|SpawnActorFromClass` "/Game/Blueprints/Items/LandscapeResources/BP_RaspberryNode.BP_RaspberryNode_C" (`KismetMathLibrary.MakeTransform` (`KismetMathLibrary.MakeVector` (.x (`self.ChosenPoint`)) (.y (`self.ChosenPoint`)) (.z (`.ImpactPoint` (`GameplayStatics.BreakHitResult` _outhit))))) "AdjustIfPossibleButAlwaysSpawn" "OverrideRootScale" null null))))))

(fn `UserConstructionScript`)