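; BP_OreSpawner is a one-shot placeholder actor that spawns an ore at its own transform, then destroys itself.
; On BeginPlay it picks randomly between CopperOre and the current ChosenOre value, storing the result back in ChosenOre.
; A valid class spawns with collision adjusted but always spawning.
; An empty pick prints a debug message instead, and the spawner is still destroyed.
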(event `self.ReceiveBeginPlay`
  (bind _output_get (set `self.ChosenOre` (`KismetArrayLibrary.Array_Random` (`|MakeArray` (`self.CopperOre`) (`self.ChosenOre`) :!type "MiningRock Class Reference"))))
  (if (!= _output_get null)
    (`|SpawnActorFromClass` _output_get (`self.GetTransform`) "AdjustIfPossibleButAlwaysSpawn" "OverrideRootScale" null null)
    (else
      (`KismetSystemLibrary.PrintString` "Empty  ore class chosen")))
  (`self.K2_DestroyActor`))

(fn `UserConstructionScript`)