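; BP_Sword is a sword weapon Blueprint that breaks and scatters destructible physics objects at a given location.
; Its CreateFields event drives a Field System component, applying radial external cluster strain to fracture, then a filtered radial linear force to push pieces outward.
; Unconnected leftover nodes hold a socket-based Niagara weapon trail and debug spheres; the other events and construction script are empty.
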(event `self.ReceiveBeginPlay`)

(event `self.CreateFields`
  (params (FieldLocation :type "Vector Structure (by ref)"))
  (bind _fieldsystem_0 (`self.FieldSystem_0`))
  (`FieldSystemComponent.ApplyPhysicsField` _fieldsystem_0 true "Field_ExternalClusterStrain" null (`RadialFalloff.SetRadialFalloff` (`self.RadialFalloff1`) 1000000.0 1.0 1.0 0.0 200.0 FieldLocation "Field_FallOff_None"))
  (`FieldSystemComponent.ApplyPhysicsField` _fieldsystem_0 true "Field_LinearForce" (`self.FieldSystemMetaDataFilter1`) (`RadialVector.SetRadialVector` (`self.RadialVector1`) 900000.0 FieldLocation)))

(fn `UserConstructionScript`)