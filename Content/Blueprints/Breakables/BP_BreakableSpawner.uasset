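; BP_BreakableSpawner is a placement actor that randomly decides which breakable, if any, appears at its location.
; On BeginPlay it picks from an array of three breakable classes and three BreakableNone entries, the repeats weighting the roll toward that option.
; A valid pick spawns at the spawner's transform, adjusted for collision but always spawning, while an empty pick spawns nothing.
; Both outcomes print a debug string.
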(event `self.ReceiveBeginPlay`
  (bind _output_get (set `self.ChosenPot` (`KismetArrayLibrary.Array_Random` (`|MakeArray` (`self.Breakable1`) (`self.Breakable2`) (`self.Breakable3`) (`self.BreakableNone`) (`self.BreakableNone`) (`self.BreakableNone`) :!type "BreakableActor Class Reference"))))
  (if (!= _output_get null)
    (`KismetSystemLibrary.PrintString` (`KismetSystemLibrary.GetClassDisplayName` _output_get))
    (`|SpawnActorFromClass` _output_get (`self.GetTransform`) "AdjustIfPossibleButAlwaysSpawn" "OverrideRootScale" null null)
    (else
      (`KismetSystemLibrary.PrintString` "Picked no class; not spawning"))))

(fn `UserConstructionScript`)