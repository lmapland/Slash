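; Roxanne character Blueprint, assembled from modular body, hair and armour components and able to show floating damage numbers.
; The construction script makes every part follow the main Mesh's animation through SetMasterPoseComponent.
; DisplayDamageWidget creates a WBP_FloatingDamage at a screen position projected from just above the actor and adds it to the viewport.
; GetHit only forwards to the parent implementation, and BeginPlay is empty.
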(event `self.ReceiveBeginPlay`)

(event `self.DisplayDamageWidget`
  (params (Amount :type "Float (single-precision)"))
  (bind _returnvalue (`|CreateWidget` (`self.DamageWidget`)))
  (bind _aswbp_floating_damage (cast `/Game/Blueprints/HUD/WBP_FloatingDamage` _returnvalue)
    (:`then`
      (`/Game/Blueprints/HUD/WBP_FloatingDamage.Setup` _aswbp_floating_damage Amount (`WidgetLayoutLibrary.ProjectWorldLocationToWidgetPosition` (`self.GetPlayerController`) (+ (`self.K2_GetActorLocation`) (0.0 0.0 100.0))))
      (`UserWidget.AddToViewport` _aswbp_floating_damage 0))
    (:`CastFailed`
      (`KismetSystemLibrary.PrintString` "Cast to FloatingDamage failed"))))

(event `HitInterface.GetHit`
  (params (ImpactPoint :type "Vector Structure (by ref)") (DamageDealt :type "Float (single-precision)") (Hitter :type "Actor Object Reference"))
  (`parent.GetHit` ImpactPoint DamageDealt Hitter))

(fn `UserConstructionScript`
  (`SkinnedMeshComponent.SetLeaderPoseComponent` (`self.EyebrowsComponent`) (`self.Mesh`) false)
  (`SkinnedMeshComponent.SetLeaderPoseComponent` (`self.BeardComponent`) (`self.Mesh`) false)
  (`SkinnedMeshComponent.SetLeaderPoseComponent` (`self.MoustacheComponent`) (`self.Mesh`) false)
  (`SkinnedMeshComponent.SetLeaderPoseComponent` (`self.SideburnComponent`) (`self.Mesh`) false)
  (`SkinnedMeshComponent.SetLeaderPoseComponent` (`self.HairComponent`) (`self.Mesh`) false)
  (`SkinnedMeshComponent.SetLeaderPoseComponent` (`self.TopknotComponent`) (`self.Mesh`) false)
  (`SkinnedMeshComponent.SetLeaderPoseComponent` (`self.LegArmourComponent`) (`self.Mesh`) false)
  (`SkinnedMeshComponent.SetLeaderPoseComponent` (`self.BootsArmourComponent`) (`self.Mesh`) false)
  (`SkinnedMeshComponent.SetLeaderPoseComponent` (`self.BeltArmourComponent`) (`self.Mesh`) false)
  (`SkinnedMeshComponent.SetLeaderPoseComponent` (`self.HelmetArmourComponent`) (`self.Mesh`) false)
  (`SkinnedMeshComponent.SetLeaderPoseComponent` (`self.ShoulderArmourComponent`) (`self.Mesh`) false)
  (`SkinnedMeshComponent.SetLeaderPoseComponent` (`self.ChestArmourComponent`) (`self.Mesh`) false)
  (`SkinnedMeshComponent.SetLeaderPoseComponent` (`self.GloveArmourComponent`) (`self.Mesh`) false)
  (`SkinnedMeshComponent.SetLeaderPoseComponent` (`self.BackArmourComponent`) (`self.Mesh`) false)
  (`SkinnedMeshComponent.SetLeaderPoseComponent` (`self.BracersArmourComponent`) (`self.Mesh`) false)
  (`SkinnedMeshComponent.SetLeaderPoseComponent` (`self.FeetComponent`) (`self.Mesh`) false)
  (`SkinnedMeshComponent.SetLeaderPoseComponent` (`self.LegsComponent`) (`self.Mesh`) false)
  (`SkinnedMeshComponent.SetLeaderPoseComponent` (`self.HandsComponent`) (`self.Mesh`) false)
  (`SkinnedMeshComponent.SetLeaderPoseComponent` (`self.ArmsComponent`) (`self.Mesh`) false)
  (`SkinnedMeshComponent.SetLeaderPoseComponent` (`self.ChestComponent`) (`self.Mesh`) false)
  (`SkinnedMeshComponent.SetLeaderPoseComponent` (`self.NeckComponent`) (`self.Mesh`) false)
  (`SkinnedMeshComponent.SetLeaderPoseComponent` (`self.FaceComponent`) (`self.Mesh`) false)
  (`SkinnedMeshComponent.SetLeaderPoseComponent` (`self.EyesComponent`) (`self.Mesh`) false))